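; Game mode Blueprint that runs a minutes-and-seconds countdown and pauses the game when time runs out.
; Tick feeds a one-second Delay, which ignores calls while pending, so the seconds variable (秒) drops about once per second.
; When seconds fall below zero they wrap to 59 and minutes (分) drop by one.
; With no minutes left, seconds reset to zero and the game pauses.
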(event EventTick
  (params (DeltaSeconds :type Float%20%28single-precision%29))
  ;[1 0 0.2312] 倒數系統
  ;;[1 1 1] 每秒秒數減一
  (Utilities|FlowControl|Delay 1.0) ; 延遲:等待所設定的時間在執行後面的節點
  (bind _output_get (Variables|Default|Set秒 (- (Variables|Default|Get秒) 1)))
  ;;[1 1 1] 當秒數為0重新設定為59
  (if (< _output_get 0) ; 判斷:當布林值為正確\n就從true出去\n為錯誤\n就從false出去
    (Variables|Default|Set秒 59)
    ;;[1 1 1] 分數大於0時分減1
    (if (> (Variables|Default|Get分) 0)
      (Variables|Default|Set分 (- (Variables|Default|Get分) 1))
      (else
        ;;[1 1 1] 分為0時秒等於59 帶秒沒有時間 將秒設為0並暫停遊戲
        (if (== (Variables|Default|Get秒) 59)
          (Variables|Default|Set秒 0)
          (Game|SetGamePaused true))))))

(fn ConstructionScript)